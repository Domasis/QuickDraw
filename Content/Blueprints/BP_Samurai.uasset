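; BP_Samurai is a sprite-based duelist in a quick-draw samurai duel, driven by the phase of GM_Duel.
; An attack during Wait shows a cross and locks further input; during Draw it finishes the round and plays a fast lunge.
; Timelines lerp the sprite for slide-in and lunge, with an event track swapping to the attack sprite and reporting success to the game mode.
; Defeat swaps the sprite, and Reset restores idle.
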(event Custom|Slide%20In
  (Components|Timeline|SetPlayRate (Variables|Default|GetSlideInAnim) 2.0)
  (bind _alpha (Timeline|SlideInAnim PlayFromStart)
    (:Update
      (Transformation|SetRelativeLocation (Variables|Default|GetPlayerSprite) (Math|Vector|Lerp(Vector) (Variables|Default|GetSlideStartPos) (Variables|Default|GetSpriteDefaultPos) _alpha) false false))))

(event Custom|Attack
  (if (not (Variables|Default|GetPressedDraw))
    (switch Utilities|FlowControl|Switch|SwitchonE_Phase (Variables|/Game/Blueprints/GM_Duel.GM_Duel_C|GetPhase (Variables|Default|GetGameModeRef))
      (:NewEnumerator1
        (CallFunction|SetCrossVisibility true)
        (Variables|Default|SetPressedDraw true))
      (:NewEnumerator2
        (Variables|Default|SetPressedDraw true)
        (Default|SetGameFinished (Variables|Default|GetGameModeRef))
        (Components|Timeline|SetPlayRate (Variables|Default|GetAttackAnim) 8.0)
        (bind _alpha (Timeline|AttackAnim PlayFromStart)
          (:Update
            (Transformation|SetRelativeLocation (Variables|Default|GetPlayerSprite) (Math|Vector|Lerp(Vector) (Variables|Default|GetSpriteDefaultPos) (Variables|/Script/Engine.SceneComponent|GetRelativeLocation (Variables|Default|GetAttackPos)) _alpha) false false))
          (:SwitchSprite
            (CallFunction|SetSprite (Variables|Default|GetAttackSprite))
            (Default|AttackedSuccessfully (Variables|Default|GetGameModeRef) (Pawn|IsPlayerControlled))))))))

(event Custom|Defeated
  (CallFunction|SetSprite (Variables|Default|GetDefeatedSprite))
  (CallFunction|SetCrossVisibility false))

(event EventBeginPlay
  (bind _asgm_duel (Utilities|Casting|CastToGM_Duel (Game|GetGameMode)))
  (Variables|Default|SetGameModeRef _asgm_duel)
  (Variables|Default|SetSpriteDefaultPos (Variables|/Script/Engine.SceneComponent|GetRelativeLocation (Variables|Default|GetPlayerSprite)))
  (CallFunction|Slidein)
  (CallFunction|SetCrossVisibility false))

(fn ConstructionScript)

(fn SetCrossVisibility
  (params (bNewVisibility :type Boolean))
  (Rendering|SetVisibility (Variables|Default|GetCross) bNewVisibility true))

(fn SetSprite
  (params (NewSprite :type Paper%20Sprite%20Object%20Reference))
  (bind _playersprite (Variables|Default|GetPlayerSprite))
  (Rendering|Components|Sprite|SetSprite (Variables|Default|GetPlayerSprite) NewSprite)
  (Rendering|Material|SetMaterial _playersprite 0 "/Paper2D/TranslucentUnlitSpriteMaterial.TranslucentUnlitSpriteMaterial")
  (Rendering|SetTranslucentSortPriority _playersprite 1))

(fn Reset
  (CallFunction|SetSprite (Variables|Default|GetIdleSprite))
  (Variables|Default|SetPressedDraw false)
  (CallFunction|Slidein))